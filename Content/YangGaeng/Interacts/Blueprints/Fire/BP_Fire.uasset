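; BP_Fire is a fire hazard that damages BPI_Damage actors and can be put out by extinguisher smoke.
; Each BP_Extinguisher_Smoke overlap on Sphere lowers LifeCount; at zero it disables collision and FX, calls EndEvent, then destroys itself after a delay.
; HitBox and SmokeBox overlaps run repeating timelines that send damage messages.
; SpawnSetting sets SmokeMode, which gates smoke damage and FX activation.
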(event `self.Sphere.OnComponentBeginOverlap`
  (params (OverlappedComponent :type "PrimitiveComponent Object Reference") (OtherActor :type "Actor Object Reference") (OtherComp :type "PrimitiveComponent Object Reference") (OtherBodyIndex :type Integer) (bFromSweep :type Boolean) (SweepResult :type "HitResult Structure (by ref)"))
  (if (`.bSuccess` (cast `/Game/YangGaeng/Interacts/Blueprints/Fire/BP_Extinguisher_Smoke` OtherActor :!pure true))
    (bind _output_get (set `self.LifeCount` (+ (`self.LifeCount`) -1)))
    (if (<= _output_get 0)
      (`PrimitiveComponent.SetCollisionEnabled` (`self.Sphere`) "NoCollision")
      (`ActorComponent.Deactivate` (`self.FX`))
      (`PrimitiveComponent.SetCollisionEnabled` (`self.SmokeBox`) "NoCollision")
      (`PrimitiveComponent.SetCollisionEnabled` (`self.HitBox`) "NoCollision")
      (`self.End Event`)
      (`KismetSystemLibrary.Delay` 6.0)
      (`self.K2_DestroyActor`))))

(event `self.HitBox.OnComponentBeginOverlap`
  (params (OverlappedComponent :type "PrimitiveComponent Object Reference") (OtherActor :type "Actor Object Reference") (OtherComp :type "PrimitiveComponent Object Reference") (OtherBodyIndex :type Integer) (bFromSweep :type Boolean) (SweepResult :type "HitResult Structure (by ref)"))
  (if (`KismetSystemLibrary.DoesImplementInterface` OtherActor "/Game/YangGaeng/Character/Blueprints/BPI_Damage.BPI_Damage_C")
    (`Timeline|Fire Damage Timeline` :!via `PlayFromStart` :!label _label
      (:`Update`
        (`/Engine/EditorBlueprintResources/StandardMacros.DoOnce` false :!label _label_2
          (:`Completed`
            (message `/Game/YangGaeng/Character/Blueprints/BPI_Damage.Apply Damage` OtherActor self))))
      (:`Finished`
        (`|ExecutionSequence`
          (:`then_0`
            (goto _label_2 :!via `Reset`))
          (:`then_1`
            (if (`PrimitiveComponent.IsOverlappingComponent` (`self.HitBox`) OverlappedComponent)
              (goto _label :!via `PlayFromStart`))))))))

(event `self.SmokeBox.OnComponentBeginOverlap`
  (params (OverlappedComponent :type "PrimitiveComponent Object Reference") (OtherActor :type "Actor Object Reference") (OtherComp :type "PrimitiveComponent Object Reference") (OtherBodyIndex :type Integer) (bFromSweep :type Boolean) (SweepResult :type "HitResult Structure (by ref)"))
  (if (and (`KismetSystemLibrary.DoesImplementInterface` OtherActor "/Game/YangGaeng/Character/Blueprints/BPI_Damage.BPI_Damage_C") (`self.SmokeMode`))
    (`Timeline|Expose Smoke Timeline` :!via `PlayFromStart` :!label _label_3
      (:`Finished`
        (message `/Game/YangGaeng/Character/Blueprints/BPI_Damage.Apply Damage` OtherActor self)
        (if (`self.IsOverlappingActor` OtherActor self)
          (goto _label_3 :!via `PlayFromStart`))))))

(event `self.SmokeBox.OnComponentEndOverlap`
  (params (OverlappedComponent :type "PrimitiveComponent Object Reference") (OtherActor :type "Actor Object Reference") (OtherComp :type "PrimitiveComponent Object Reference") (OtherBodyIndex :type Integer))
  (goto _label_3 :!via `Stop`))

(fn `SpawnSetting`
  (params (bIsAdditionSmoke :type Boolean))
  (bind _output_get (set `self.SmokeMode` bIsAdditionSmoke))
  (`ActorComponent.SetActive` (`self.FX`) _output_get false))

(fn `UserConstructionScript`)