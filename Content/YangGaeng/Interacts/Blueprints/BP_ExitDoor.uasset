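; BP_ExitDoor is an interactable exit door that swings open once when a character interacts with it.
; BeginPlay registers the door and frame as highlight meshes and stops the door sound.
; A CanOperate guard blocks repeat use, then a timeline yaws the door mesh to 90 degrees while the sound plays.
; When the timeline finishes, it calls EndEvent.
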(event `self.ReceiveBeginPlay`
  (`parent.ReceiveBeginPlay`)
  (set `self.HighlightMeshes` (`|MakeArray` (`self.Door`) (`self.DoorFrame`)))
  (`AudioComponent.Stop` (`self.DoorSound`)))

(event `self.Interact Event`
  (params (Character :type "/Game/YangGaeng/Character/Blueprints/BP_PlayerLevelCharacter Object Reference") (`bIsUI Expression` :type Boolean))
  (if (`self.bCanOperate`)
    (set `self.bCanOperate` false)
    (`parent.Interact Event` Character `bIsUI Expression`)
    (`|ExecutionSequence`
      (:`then_0`
        (bind (_direction _ratio) (`Timeline|Door Open Timeline`)
          (:`Update`
            (`SceneComponent.K2_SetRelativeRotation` (`self.SM_door`) (`KismetMathLibrary.MakeRotator` 0.0 0.0 (* _ratio 90.0)) false false))
          (:`Finished`
            (`self.End Event`))))
      (:`then_1`
        (`AudioComponent.Play` (`self.DoorSound`) 0.0)))))

(fn `UserConstructionScript`
  (`parent.UserConstructionScript`))