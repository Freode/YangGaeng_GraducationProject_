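; BP_Stair is an interactable stair that applies a force to the player character when used.
; It registers StairFrame as its highlight mesh on BeginPlay.
; InteractEvent, gated by CanOperate, calls the parent logic, then pushes the first player character overlapping InteractBox using the Direction component's relative location as the force vector.
; If a player was found, EndEvent follows after a fixed delay.
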(event `self.ReceiveBeginPlay`
  (`parent.ReceiveBeginPlay`)
  (set `self.HighlightMeshes` (`|MakeArray` (`self.StairFrame`))))

(event `self.Interact Event`
  (params (Character :type "/Game/YangGaeng/Character/Blueprints/BP_PlayerLevelCharacter Object Reference") (`bIsUI Expression` :type Boolean))
  (bind _overlappingactors (`PrimitiveComponent.GetOverlappingActors` (`self.InteractBox`) "/Game/YangGaeng/Character/Blueprints/BP_PlayerLevelCharacter.BP_PlayerLevelCharacter_C"))
  (if (`self.bCanOperate`)
    (set `self.bCanOperate` false)
    (`parent.Interact Event` Character `bIsUI Expression`)
    (if (> (`KismetArrayLibrary.Array_Length` _overlappingactors) 0)
      (`CharacterMovementComponent.AddForce` (`Character.CharacterMovement` (cast `/Game/YangGaeng/Character/Blueprints/BP_PlayerLevelCharacter` (`|GetArrayItem` _overlappingactors) :!pure true)) (`SceneComponent.RelativeLocation` (`self.direction`)))
      (`KismetSystemLibrary.Delay` 5.0)
      (`self.End Event`))))

(fn `UserConstructionScript`
  (`parent.UserConstructionScript`))