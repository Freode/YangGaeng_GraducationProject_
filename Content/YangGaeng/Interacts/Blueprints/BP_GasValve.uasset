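; Interactable gas valve that can be operated while CanOperate is true, registering its Valve mesh for highlighting on BeginPlay.
; Interacting clears CanOperate, runs the parent interact logic and plays ValveRockTimeline.
; The timeline drives the whole actor's pitch as its track value times 90 degrees with yaw fixed at 90, then calls EndEvent when finished.
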(event `self.ReceiveBeginPlay`
  (`parent.ReceiveBeginPlay`)
  (set `self.HighlightMeshes` (`|MakeArray` (`self.Valve`))))

(event `self.Interact Event`
  (params (Character :type "/Game/YangGaeng/Character/Blueprints/BP_PlayerLevelCharacter Object Reference") (`bIsUI Expression` :type Boolean))
  (if (`self.bCanOperate`)
    (set `self.bCanOperate` false)
    (`parent.Interact Event` Character `bIsUI Expression`)
    (bind (_direction _newtrack_0) (`Timeline|ValveRockTimeline`)
      (:`Update`
        (`self.K2_SetActorRotation` (`KismetMathLibrary.MakeRotator` 0.0 (* _newtrack_0 90.0) 90.0)))
      (:`Finished`
        (`self.End Event`)))))

(fn `UserConstructionScript`
  (`parent.UserConstructionScript`))