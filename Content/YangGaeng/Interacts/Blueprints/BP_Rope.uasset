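; BP_Rope is an interactable rope actor that visually lowers itself when RopeDown fires.
; RopeDown prints a debug string, runs a timed MoveComponentTo downward that feeds world X/Y into a relative target, and plays the DescendingRope timeline.
; The timeline's Velocity track drives the Cylinder's world Z scale, stretching the thin mesh as rope.
; InteractEvent is empty, and nothing in this graph calls RopeDown.
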(event `self.Interact Event`
  (params (Character :type "/Game/YangGaeng/Character/Blueprints/BP_PlayerLevelCharacter Object Reference") (`bIsUI Expression` :type Boolean)))

(event `Rope Down`
  (bind (_returnvalue_x _returnvalue_y) (`KismetMathLibrary.BreakVector` (`SceneComponent.K2_GetComponentLocation` (`self.Cylinder`))))
  (`KismetSystemLibrary.PrintString` "Hello")
  (`KismetSystemLibrary.MoveComponentTo` null (`KismetMathLibrary.MakeVector` _returnvalue_x _returnvalue_y -150.0) (struct) false false 5.0)
  (bind (_direction _velocity) (`Timeline|Descending Rope`)
    (:`Update`
      (`SceneComponent.SetWorldScale3D` (`self.Cylinder`) (`KismetMathLibrary.MakeVector` 0.05 0.05 (* _velocity 60.0))))))

(fn `UserConstructionScript`
  (`parent.UserConstructionScript`))