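; BPC_Count is a component that acts as a simple time-based trigger for interactable objects.
; Each Tick it adds delta time to Count and sets IsOperate once Count exceeds Threshold.
; DoOnceOperate returns true and clears the flag when it is set, otherwise false.
; Count is never reset, so the flag is raised again on every Tick after the threshold is passed.
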(event `self.ReceiveTick`
  (params (DeltaSeconds :type "Float (single-precision)"))
  (set `self.Count` (+ DeltaSeconds (`self.Count`)))
  (if (> (`self.Count`) (`self.Threshold`))
    (set `self.bIsOperate` true)))

(fn `DoOnceOperate`
  (returns (bOperate :type Boolean))
  (if (`self.bIsOperate`)
    (set `self.bIsOperate` false)
    (return true)
    (else
      (return false))))