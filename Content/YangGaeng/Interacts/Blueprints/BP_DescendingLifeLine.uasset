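; BP_DescendingLifeLine is an interactable descending lifeline that swings around and lowers a rope along with the player.
; InteractEvent plays a timeline that yaws the actor toward -90 degrees and checks the Box for a player on every update.
; An overlapping player is moved to the rope's relative Z, while a second timeline stretches and lowers SMRope through MoveComponentTo calls reissued each update.
; A BP_Rope RopeDown call is left unconnected.
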(event `self.Interact Event`
  (params (Character :type "/Game/YangGaeng/Character/Blueprints/BP_PlayerLevelCharacter Object Reference") (`bIsUI Expression` :type Boolean))
  (bind _sm_rope (`self.SM_Rope`))
  (bind _overlappingactors (`PrimitiveComponent.GetOverlappingActors` (`self.Box`) "/Game/YangGaeng/Character/Blueprints/BP_PlayerLevelCharacter.BP_PlayerLevelCharacter_C"))
  (bind (_relativelocation_x _relativelocation_y _relativelocation_z) (`KismetMathLibrary.BreakVector` (`SceneComponent.RelativeLocation` _sm_rope)))
  (bind _asbp_player_level_character (cast `/Game/YangGaeng/Character/Blueprints/BP_PlayerLevelCharacter` (`|GetArrayItem` _overlappingactors) :!pure true))
  (bind (_returnvalue_x _returnvalue_y) (`KismetMathLibrary.BreakVector` (`SceneComponent.K2_GetComponentLocation` (`Character.CapsuleComponent` _asbp_player_level_character))))
  (bind (_direction _ratio) (`Timeline|Timeline`)
    (:`Update`
      (`self.K2_SetActorRotation` (`KismetMathLibrary.MakeRotator` 0.0 0.0 (* _ratio -90.0)))
      (if (> (`KismetArrayLibrary.Array_Length` _overlappingactors) 0)
        (`|ExecutionSequence`
          (:`then_0`
            (`KismetSystemLibrary.MoveComponentTo` (`Actor.RootComponent` _asbp_player_level_character) (`KismetMathLibrary.MakeVector` _returnvalue_x _returnvalue_y _relativelocation_z) (struct) false false 5.0))
          (:`then_1`
            (bind (_direction_2 _velocity) (`Timeline|Timeline_0`)
              (:`Update`
                (`SceneComponent.SetRelativeScale3D` _sm_rope (`KismetMathLibrary.MakeVector` 0.1 0.1 _velocity))
                (`KismetSystemLibrary.MoveComponentTo` _sm_rope (`KismetMathLibrary.MakeVector` _relativelocation_x _relativelocation_y -500.0) (struct) false false 2.0)))))))))

(fn `UserConstructionScript`
  (`parent.UserConstructionScript`))