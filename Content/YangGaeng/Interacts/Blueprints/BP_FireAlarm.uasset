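; BP_FireAlarm is an interactable fire alarm that sounds its alarm audio when a character uses it.
; It stops AlarmAudio on BeginPlay so the alarm starts silent.
; InteractEvent checks and clears CanOperate, runs the parent interaction and EndEvent, then plays the audio.
; Nothing in this Blueprint sets CanOperate back to true or stops the alarm once triggered.
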(event `self.ReceiveBeginPlay`
  (`AudioComponent.Stop` (`self.AlarmAudio`)))

(event `self.Interact Event`
  (params (Character :type "/Game/YangGaeng/Character/Blueprints/BP_PlayerLevelCharacter Object Reference") (`bIsUI Expression` :type Boolean))
  (if (`self.bCanOperate`)
    (set `self.bCanOperate` false)
    (`parent.Interact Event` Character `bIsUI Expression`)
    (`self.End Event`)
    (`AudioComponent.Play` (`self.AlarmAudio`) 0.0)))

(fn `UserConstructionScript`
  (`parent.UserConstructionScript`))