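; BP_Interact_Base is a base interactable actor that can be highlighted, show an explanation and advance an interaction sequence.
; InteractEvent optionally shows its InteractKind explanation through the player character's gameplay widget.
; HighlightEvent sets a Highlight material scalar on the highlight meshes, enables box collision and marks it operable.
; EndEvent clears the highlight, disables collision and tells the BP_Interact_Sequence found by class to run the next interaction.
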(event `Interact Event`
  (params (Character :type "/Game/YangGaeng/Character/Blueprints/BP_PlayerLevelCharacter Object Reference") (`bIsUI Expression` :type Boolean))
  ;[1 1 1] ui
  (if `bIsUI Expression`
    (`/Game/YangGaeng/UI/WG_GamePlay.InformationExplaination` (`/Game/YangGaeng/Character/Blueprints/BP_PlayerLevelCharacter.WG GamePlay` (cast `/Game/YangGaeng/Character/Blueprints/BP_PlayerLevelCharacter` (`GameplayStatics.GetPlayerPawn` 0) :!pure true)) (`self.InteractKind`))))

(event `Highlight Event`
  (`self.SetHighlight` (`self.HighlightMeshes`) true)
  (`PrimitiveComponent.SetCollisionEnabled` (`self.Box`) "QueryAndPhysics")
  (set `self.bCanOperate` true))

(event `End Event`
  (`self.SetHighlight` (`self.HighlightMeshes`))
  (`PrimitiveComponent.SetCollisionEnabled` (`self.Box`) "NoCollision")
  (bind _returnvalue (`GameplayStatics.GetActorOfClass` "/Game/YangGaeng/Interacts/Blueprints/BP_Interact_Sequence.BP_Interact_Sequence_C"))
  (`/Game/YangGaeng/Interacts/Blueprints/BP_Interact_Sequence.Next Interact Event` _returnvalue))

(fn `SetHighlight`
  (params (Meshes :type "Array of StaticMeshComponent Object Reference") (bIsHighlight :type Boolean))
  (for _array_element Meshes
    (`MeshComponent.SetScalarParameterValueOnMaterials` _array_element "Highlight" (`KismetMathLibrary.SelectFloat` 1.0 0.0 bIsHighlight)))
  (return))

(fn `UserConstructionScript`)