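; BP_Elevator is an interactable elevator that closes its doors around the player when used.
; InteractEvent runs only while CanOperate is set, clears that flag, calls the parent, then plays a door-close timeline.
; Each timeline update nudges both doors in opposite directions and snaps the first player character overlapping Box to Direction's location with a fixed rotation.
; When the timeline finishes, it calls EndEvent.
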(event `self.Interact Event`
  (params (Character :type "/Game/YangGaeng/Character/Blueprints/BP_PlayerLevelCharacter Object Reference") (`bIsUI Expression` :type Boolean))
  (if (`self.bCanOperate`)
    (set `self.bCanOperate` false)
    (`parent.Interact Event` Character `bIsUI Expression`)
    (bind (_direction _close_velocity) (`Timeline|Door Close TImeline` :!via `PlayFromStart`)
      (:`Update`
        (`SceneComponent.K2_AddRelativeLocation` (`self.SM_Door_Right`) (`KismetMathLibrary.MakeVector` (* _close_velocity 4.5)) false false)
        (`SceneComponent.K2_AddRelativeLocation` (`self.SM_Door_Left`) (`KismetMathLibrary.MakeVector` (* _close_velocity -4.5)) false false)
        (`KismetSystemLibrary.MoveComponentTo` (`Actor.RootComponent` (cast `/Game/YangGaeng/Character/Blueprints/BP_PlayerLevelCharacter` (`|GetArrayItem` (`PrimitiveComponent.GetOverlappingActors` (`self.Box`) "/Game/YangGaeng/Character/Blueprints/BP_PlayerLevelCharacter.BP_PlayerLevelCharacter_C")) :!pure true)) (`SceneComponent.K2_GetComponentLocation` (`self.direction`)) (struct :`Yaw` 180.0) false false 0.01))
      (:`Finished`
        (`self.End Event`)))))

(fn `UserConstructionScript`
  (`parent.UserConstructionScript`))